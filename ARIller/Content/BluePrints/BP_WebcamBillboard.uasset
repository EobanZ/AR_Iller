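; BP_WebcamBillboard is an actor that shows a webcam video feed on a billboard component.
; On BeginPlay it applies a dynamic M_Webcam material and passes its Camera, Billboard and Cube components to C++, where the camera's FOV and ratio are adjusted.
; Each OnNextVideoFrame event feeds VideoTexture into the material's Texture parameter.
; The construction script sets the root's world location and rotation to defaults.
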(event `self.ReceiveBeginPlay`
  (bind _billboard (`self.Billboard`))
  (bind _returnvalue (`PrimitiveComponent.CreateDynamicMaterialInstance` _billboard 0 "/Game/Materials/M_Webcam.M_Webcam"))
  (`PrimitiveComponent.SetMaterial` _billboard 0 _returnvalue)
  (set `self.DynamicMaterial` _returnvalue)
  ;[1 1 1] Sets the camera reference in the c++ code to change fov and ratio
  (`self.SetCameraReference` (`self.Camera`))
  (`self.SetBillboardReference` (`self.Billboard`))
  (`self.SetCubeReference` (`self.Cube`)))

(event `self.OnNextVideoFrame`
  (`MaterialInstanceDynamic.SetTextureParameterValue` (`self.DynamicMaterial`) "Texture" (`self.VideoTexture`)))

(event `self.ReceiveTick`
  (params (DeltaSeconds :type "Float (single-precision)")))

(fn `UserConstructionScript`
  (`SceneComponent.K2_SetWorldLocationAndRotation` :`self` (`self.DefaultSceneRoot`)))